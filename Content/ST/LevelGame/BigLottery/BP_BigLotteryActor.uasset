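; BP_BigLotteryActor is a Big Lottery level actor that reacts to projectile hits by moving vertically and can trigger a force field.
; A BP_Projectile overlapping TriggerBox plays a timeline that lowers the actor by per-update offsets from its current location.
; When that finishes, Up either fires the ForceField's CETrigger if the actor is triggered, or plays a second, half-scaled timeline that raises it.
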(event `CustomEvent_0`
  (params (OverlappedComponent :type "PrimitiveComponent Object Reference") (OtherActor :type "Actor Object Reference") (OtherComp :type "PrimitiveComponent Object Reference") (OtherBodyIndex :type Integer) (bFromSweep :type Boolean) (SweepResult :type "HitResult Structure (by ref)"))
  (bind (_returnvalue_x _returnvalue_y _returnvalue_z) (`KismetMathLibrary.BreakVector` (`self.K2_GetActorLocation`)))
  (bind _asbp_projectile (cast `/Game/ST/Actors/BP_Projectile` OtherActor))
  (`/Engine/EditorBlueprintResources/StandardMacros.IsValid` _asbp_projectile
    (:`Is Valid`
      (bind (_direction _tl_goup) (`Timeline|Timeline_0`)
        (:`Update`
          (`self.K2_SetActorLocation` (`KismetMathLibrary.MakeVector` _returnvalue_x _returnvalue_y (- _returnvalue_z (* _tl_goup 1.0)))))
        (:`Finished`
          (`self.Up` OverlappedComponent OtherActor OtherComp OtherBodyIndex))))))

(event `self.ReceiveBeginPlay`
  (`|ExecutionSequence`
    (:`then_0`
      (add `PrimitiveComponent.OnComponentBeginOverlap` (`self.TriggerBox`) (delegate `CustomEvent_0`)))))

(event `Up`
  (params (OverlappedComponent :type "PrimitiveComponent Object Reference") (OtherActor :type "Actor Object Reference") (OtherComp :type "PrimitiveComponent Object Reference") (OtherBodyIndex :type Integer))
  (bind (_returnvalue_x _returnvalue_y _returnvalue_z) (`KismetMathLibrary.BreakVector` (`self.K2_GetActorLocation`)))
  (bind _forcefield (`self.ForceField`))
  (bind _returnvalue (`self.GetIsTrigged`))
  (if _returnvalue
    (`/Engine/EditorBlueprintResources/StandardMacros.IsValid` _forcefield
      (:`Is Valid`
        (`/Engine/EditorResources/FieldNodes/FS_MasterField.CE_Trigger` _forcefield)))
    (else
      (bind _asbp_projectile (cast `/Game/ST/Actors/BP_Projectile` OtherActor))
      (`/Engine/EditorBlueprintResources/StandardMacros.IsValid` _asbp_projectile
        (:`Is Valid`
          (bind (_direction _tl_goup) (`Timeline|Timeline`)
            (:`Update`
              (`self.K2_SetActorLocation` (`KismetMathLibrary.MakeVector` _returnvalue_x _returnvalue_y (+ _returnvalue_z (* _tl_goup 0.5)))))))))))

(fn `UserConstructionScript`)