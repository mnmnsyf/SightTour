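; Level-transition trigger that moves the player between streamed levels behind a loading widget.
; StartLevelEvent arms it and forwards the event to NextLevelActor via BP_LevelInterface.
; Once armed, SightTourCharacter overlap shows WBP_Loading, waits, streams in the next level, teleports to its tagged PlayerStart and unloads the current one.
; When both level names match, it parks the player at InitPosition and unloads before reloading.
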(event `/Game/ST/LevelGame/BP_LevelInterface.StartLevelEvent`
  (bind _nextlevelactor (`self.NextLevelActor`))
  (set `self.bOpenCheck` true)
  (`/Engine/EditorBlueprintResources/StandardMacros.IsValid` _nextlevelactor
    (:`Is Valid`
      (bind _asbp_level_interface (cast `/Game/ST/LevelGame/BP_LevelInterface` _nextlevelactor))
      (`/Game/ST/LevelGame/BP_LevelInterface.StartLevelEvent` _asbp_level_interface))))

(event `self.TriggerBox.OnComponentBeginOverlap`
  (params (OverlappedComponent :type "PrimitiveComponent Object Reference") (OtherActor :type "Actor Object Reference") (OtherComp :type "PrimitiveComponent Object Reference") (OtherBodyIndex :type Integer) (bFromSweep :type Boolean) (SweepResult :type "HitResult Structure (by ref)"))
  (bind _returnvalue (`GameplayStatics.GetPlayerController` 0))
  (bind _returnvalue_2 (`GameModeBase.K2_FindPlayerStart` (`GameplayStatics.GetGameMode`) (`GameplayStatics.GetPlayerController` 0) "InitPosition"))
  (if (`self.bOpenCheck`)
    (cast `SightTourCharacter` OtherActor)
    (bind _returnvalue_3 (`|CreateWidget` "/Game/UI/Loading/WBP_Loading.WBP_Loading_C"))
    (`UserWidget.AddToViewport` _returnvalue_3 0)
    (`KismetSystemLibrary.Delay` 3.0)
    (if (== (`self.CurrentLevelName`) (`self.NextLevelName`))
      (`self.K2_TeleportTo` (`GameplayStatics.GetPlayerPawn` 0) (`self.K2_GetActorLocation` _returnvalue_2) (`self.K2_GetActorRotation` _returnvalue_2))
      (`GameplayStatics.UnloadStreamLevel` (`self.CurrentLevelName`))
      (`GameplayStatics.LoadStreamLevel` (`self.NextLevelName`) true)
      (bind _asplayer_start (cast `PlayerStart` (`GameModeBase.K2_FindPlayerStart` (`GameplayStatics.GetGameMode`) (`GameplayStatics.GetPlayerController` 0) (`self.NextPlayerStartTag`))))
      (`self.K2_TeleportTo` (`GameplayStatics.GetPlayerPawn` 0) (`self.K2_GetActorLocation` _asplayer_start) (`self.K2_GetActorRotation` _asplayer_start))
      (`Widget.RemoveFromParent` _returnvalue_3)
      (else
        (`GameplayStatics.LoadStreamLevel` (`self.NextLevelName`) true)
        (`Widget.RemoveFromParent` _returnvalue_3)
        (`WidgetBlueprintLibrary.SetInputMode_GameOnly` _returnvalue)
        (bind _asplayer_start_2 (cast `PlayerStart` (`GameModeBase.K2_FindPlayerStart` (`GameplayStatics.GetGameMode`) _returnvalue (`self.NextPlayerStartTag`))))
        (`self.K2_TeleportTo` (`GameplayStatics.GetPlayerPawn` 0) (`self.K2_GetActorLocation` _asplayer_start_2) (`self.K2_GetActorRotation` _asplayer_start_2))
        (`KismetSystemLibrary.Delay` 0.1)
        (`GameplayStatics.UnloadStreamLevel` (`self.CurrentLevelName`))))))

(fn `UserConstructionScript`)